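; Aiden character Blueprint with a body built from modular parts, including feet, legs, torso, face and hair.
; The construction script calls EnableMasterPose on the feet, legs and torso to set up master-pose animation.
; The event graph has no active logic: its events are empty, and leftover custom-depth rendering and aim-pitch debug print nodes are disconnected.
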(event EventBeginPlay)

(event Collision|EventActorBeginOverlap
  (params (OtherActor :type Actor%20Object%20Reference)))

(event EventTick
  (params (DeltaSeconds :type Float%20%28single-precision%29)))

(fn ConstructionScript
  (Class|AidenCharacter|EnableMasterPose (Variables|Default|GetFeet))
  (Class|AidenCharacter|EnableMasterPose (Variables|Default|GetLegs))
  (Class|AidenCharacter|EnableMasterPose (Variables|Default|GetTorso)))