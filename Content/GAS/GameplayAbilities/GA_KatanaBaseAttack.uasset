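; GA_KatanaBaseAttack is a Gameplay Ability for the katana's base combo attack.
; On activation it commits, calls BaseAttack and plays the attack montage from the section named by CurrentCombo.
; The Montage.NextAttackCheck event starts an input wait; a press applies GE_Test to that event's target data and cancels the ability.
; The Montage.EndAttackCheck event resets the combo and ends the ability.
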(event Ability|EventActivateAbility
  (Ability|CommitAbility)
  (Class|KatanaBaseAttack|BaseAttack)
  (|PlayMontageandWaitProxy "None" "/Game/Anim/AM_Katana_Attack.AM_Katana_Attack" 1.0 (Utilities|String|StringToName (Utilities|String|ToString(Text) (Utilities|Text|FormatText "Attack{#}" (Variables|Default|GetCurrentCombo)))) true 1.0 0.0 false
    (:then
      (Utilities|FlowControl|Sequence
        (:then_0
          (bind _payload (Ability|Tasks|WaitGameplayEvent "(TagName=\"Montage.NextAttackCheck\")" 0 true)
            (:EventReceived
              (Ability|Tasks|WaitInputPress false
                (:OnPress
                  (GameplayEffects|ApplyGameplayEffectToTarget (.TargetData (Utilities|Struct|BreakGameplayEventData _payload)) "/Game/GAS/GameplayAbilities/GE_Test.GE_Test_C" 1 1)
                  (Ability|CancelAbility))))))
        (:then_1
          (Ability|Tasks|WaitGameplayEvent "(TagName=\"Montage.EndAttackCheck\")" 0 true
            (:EventReceived
              (Class|KatanaBaseAttack|ResetCombo)
              (Ability|EndAbility))))))))