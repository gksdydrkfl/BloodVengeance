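; GA_HitReact is a gameplay ability that plays the owning avatar's hit reaction.
; On activation it applies GE_HitReact to the owner, stores the handle, and plays the montage the avatar returns from GetHitReactMontage.
; When the montage blends out, is interrupted or is cancelled, it removes the effect by handle and ends the ability.
; Its own GetDeathMontage and GetHitReactMontage functions are empty.
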(event Ability|EventActivateAbility
  (bind _returnvalue (Ability|ApplyGameplayEffectToOwner "/Game/GAS/GameplayAbilities/Common/GE_HitReact.GE_HitReact_C"))
  (Variables|Default|SetActive%20GE%20Hit%20React _returnvalue)
  (bind _returnvalue_2 (Class|CombatInterface|GetHitReactMontage(Message) (Ability|GetAvatarActorfromActorInfo)))
  (|PlayMontageandWaitProxy "None" _returnvalue_2 1.0 "None" true 1.0 0.0 false
    (:OnBlendOut
      _)
    (:OnInterrupted
      _)
    (:OnCancelled
      _))
  (Ability|RemoveGameplayEffectFromOwnerWithHandle (Variables|Default|GetActive%20GE%20Hit%20React))
  (Ability|EndAbility))

(event Ability|EventOnEndAbility
  (params (bWasCancelled :type Boolean)))

(fn GetDeathMontage
  (return 0))

(fn GetHitReactMontage
  (return 0))