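; Gameplay ability for Aiden's katana base attack, playing one step of a montage-driven combo.
; On activation it commits, requires a valid katana, calls BaseAttack, updates motion warping and plays the montage section named from the current combo count.
; Montage gameplay events control the flow: a press after the next-attack check ends the ability without resetting the combo, while the end-attack check resets the combo and ends it.
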(event Ability|EventActivateAbility
  (Ability|CommitAbility)
  (bind _returnvalue (Class|KatanaBaseAttack|GetKatana))
  (Utilities|IsValid _returnvalue
    (:Is%20Valid
      (Class|KatanaBaseAttack|BaseAttack)
      (Class|KatanaBaseAttack|UpdateMotionWarping)
      (|PlayMontageandWaitProxy "None" "/Game/Characters/Aiden/Animations/Katana/Attack/Montage/AM_Katana_ComboAttack2.AM_Katana_ComboAttack2" 1.0 (Utilities|String|StringToName (Utilities|String|ToString(Text) (Utilities|Text|FormatText "Attack{#}" (Variables|Default|GetCurrentCombo)))) true 1.0 0.0 false
        (:then
          (Utilities|FlowControl|Sequence
            (:then_0
              (Ability|Tasks|WaitGameplayEvent "(TagName=\"Montage.NextAttackCheck\")" 0 true
                (:EventReceived
                  (Ability|Tasks|WaitInputPress false
                    (:OnPress
                      (Ability|EndAbility))))))
            (:then_1
              (Ability|Tasks|WaitGameplayEvent "(TagName=\"Montage.EndAttackCheck\")" 0 true
                (:EventReceived
                  (Class|KatanaBaseAttack|ResetCombo)
                  (Ability|EndAbility))))))))
    (:Is%20Not%20Valid
      (Ability|EndAbility))))