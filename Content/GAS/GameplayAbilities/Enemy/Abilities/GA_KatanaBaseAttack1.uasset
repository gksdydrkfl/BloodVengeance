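; GA_KatanaBaseAttack1 is an enemy gameplay ability for a katana combo attack.
; On activation it commits, calls BaseAttack and UpdateMotionWarping, then plays the AM_Enemy_Test montage from the section named by CurrentCombo.
; The NextAttackCheck montage event starts an input-press wait that ends the ability without resetting the combo.
; The EndAttackCheck event resets the combo and ends the ability.
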(event Ability|EventActivateAbility
  (Ability|CommitAbility)
  (Class|KatanaBaseAttack|BaseAttack)
  (Class|KatanaBaseAttack|UpdateMotionWarping)
  (|PlayMontageandWaitProxy "None" "/Game/Characters/Enemy/Animations/Montage/Soldier/AM_Enemy_Test.AM_Enemy_Test" 1.0 (Utilities|String|StringToName (Utilities|String|ToString(Text) (Utilities|Text|FormatText "Attack{#}" (Variables|Default|GetCurrentCombo)))) true 1.0 0.0 false
    (:then
      (Utilities|FlowControl|Sequence
        (:then_0
          (Ability|Tasks|WaitGameplayEvent "(TagName=\"Montage.NextAttackCheck\")" 0 true
            (:EventReceived
              (Ability|Tasks|WaitInputPress false
                (:OnPress
                  (Ability|EndAbility))))))
        (:then_1
          (Ability|Tasks|WaitGameplayEvent "(TagName=\"Montage.EndAttackCheck\")" 0 true
            (:EventReceived
              (Class|KatanaBaseAttack|ResetCombo)
              (Ability|EndAbility))))))))